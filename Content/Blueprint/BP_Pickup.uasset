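; BP_Pickup is an interactable object that can be picked up and attached to the component supplied by whoever uses it.
; On Interact, it turns off the Cube's collision and physics, attaches to the passed UseComponent and snaps the actor to that component's world transform.
; Engage and Disengage show and hide an arrow indicator, and all three events print debug messages.
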(event EventInteract
  (params (Instigator :type Object%20Object%20Reference) (Message :type String) (UseComponent :type Scene%20Component%20Object%20Reference))
  (bind _cube (Variables|Default|GetCube))
  (Development|PrintString (Utilities|String|Append "Instigator: " (Utilities|GetDisplayName Instigator) " 
Interact Event: " Message))
  (Collision|SetCollisionEnabled _cube "NoCollision")
  (Physics|SetSimulatePhysics _cube false)
  (Transformation|AttachComponentToComponent UseComponent "None" "KeepRelative" "KeepRelative" "KeepRelative" true)
  (Transformation|SetActorTransform (Transformation|GetWorldTransform UseComponent)))

(event EventEngage
  (Development|PrintString (Utilities|String|Append "Self: " (Utilities|GetDisplayName self) " 
Event: ENGAGED") true true "(R=1.000000,G=0.000000,B=0.000000,A=1.000000)")
  (Development|SetHiddeninGame (Variables|Default|GetArrow1) false false))

(event EventDisengage
  (Development|PrintString (Utilities|String|Append "Self: " (Utilities|GetDisplayName self) " 
Event: DISENGAGED") true true "(R=1.000000,G=0.578253,B=0.000000,A=1.000000)")
  (Development|SetHiddeninGame (Variables|Default|GetArrow1) true false))

(fn ConstructionScript)