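; Dev component that shows debug stats on screen each tick, toggled by the TickRate and CharacterInfo flags.
; StatTickRate prints FPS derived from world delta seconds, with the flag controlling only the screen output.
; StatCharacters finds all actors of player 0's controller class and prints each controller ID with its controlled pawn's name.
; Each message lasts one frame's delta time, so the readout refreshes continuously.
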(event EventBeginPlay)

(event EventTick
  (params (DeltaSeconds :type Float%20%28single-precision%29))
  (Utilities|FlowControl|Sequence
    (:then_0
      (CallFunction|StatTickRate (Variables|Default|GettickRate)))
    (:then_2
      (CallFunction|StatCharacters (Variables|Default|GetcharacterInfo)))))

(fn StatCharacters
  (params (show? :type Boolean))
  (if show?
    (bind _outactors (Actor|GetAllActorsOfClass (Utilities|GetClass (Game|GetPlayerController 0))))
    (for _array_element _outactors
      (Development|PrintString (Utilities|String|Append "Controller  " (Utilities|String|ToString(Integer) (Class|GameplayStatics|GetPlayerControllerID _array_element)) " - " (Utilities|GetObjectName (Pawn|GetControlledPawn _array_element))) true true "(R=0.000000,G=0.660000,B=1.000000,A=1.000000)" (Utilities|Time|GetWorldDeltaSeconds)))
    (else
      (return))))

(fn StatTickRate
  (params (show? :type Boolean))
  (bind _returnvalue (Utilities|Time|GetWorldDeltaSeconds))
  (Development|PrintString (Utilities|String|Append "FPS: " (Utilities|String|ToString(Float) (/ 1.0 _returnvalue))) show? true "(R=1.000000,G=0.000000,B=0.740991,A=1.000000)" _returnvalue))