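; Actor component that gives its owner health and handles its death with kill credit.
; OnDamaged subtracts health and accumulates damage per causer in parallel causer and damage arrays.
; While the owner survives, a retriggerable four-second delay clears the causer list after damage stops.
; At zero health, OnDeath sends the last causer a kill message with its accumulated damage, then destroys the owner.
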(event EventOnDamaged
  (params (Damage :type Float%20%28single-precision%29) (DamageType :type Damage%20Type%20Object%20Reference) (InstigatedBy :type Controller%20Object%20Reference) (DamageCauser :type Actor%20Object%20Reference))
  (bind _damagecausers (Variables|Default|GetDamageCausers))
  (bind _damagecausersdamage (Variables|Default|GetDamageCausersDamage))
  (bind _returnvalue (Utilities|Array|Length _damagecausers))
  (bind _returnvalue_2 (Utilities|Array|ContainsItem _damagecausers DamageCauser))
  (bind _returnvalue_3 (Utilities|Array|FindItem _damagecausers DamageCauser))
  (bind _returnvalue_4 (select _returnvalue_2 _returnvalue_3 _returnvalue))
  (Variables|Default|SetLastDamageCauser DamageCauser)
  (Variables|Default|SetHealth (- (Variables|Default|GetHealth) Damage))
  (Utilities|Array|SetArrayElem _damagecausers _returnvalue_4 DamageCauser true)
  (Utilities|Array|SetArrayElem _damagecausersdamage _returnvalue_4 (select _returnvalue_2 (+ (Utilities|Array|Get(acopy) _damagecausersdamage _returnvalue_4) Damage) Damage) true)
  (if (not (<= (Variables|Default|GetHealth) 0.0))
    (Utilities|FlowControl|RetriggerableDelay 4.0)
    (Utilities|Array|Clear (Variables|Default|GetDamageCausers))
    (Development|PrintString "Damage Causers \\n Cleared")
    (else
      (CallFunction|OnDeath Damage 0 0 (Variables|Default|GetLastDamageCauser)))))

(event EventOnDeath
  (params (Damage :type Float%20%28single-precision%29) (DamageType :type Damage%20Type%20Object%20Reference) (InstigatedBy :type Controller%20Object%20Reference) (DamageCauser :type Actor%20Object%20Reference))
  (bind _returnvalue (Components|GetOwner))
  (bind _lastdamagecauser (Variables|Default|GetLastDamageCauser))
  (Class|BPInterKillable|OnKill(Message) _lastdamagecauser (Utilities|Array|Get(acopy) (Variables|Default|GetDamageCausersDamage) (Utilities|Array|FindItem (Variables|Default|GetDamageCausers) _lastdamagecauser)) (Variables|Default|GetController) _returnvalue)
  (Actor|DestroyActor _returnvalue))