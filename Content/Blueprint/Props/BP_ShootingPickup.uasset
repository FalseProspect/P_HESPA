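; Shooting pickup prop that attaches to whoever interacts with it and fires hitscan damage while held.
; Reach interact stores the invoker's controller, disables physics and collision, and snaps the pickup to the invoker's component.
; Held Start runs a looping line trace from the Arrow plus a mesh-sliding timeline; Stop clears both.
; Drop restores physics and calls DetachFromActor on the stored parent actor rather than the pickup.
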(event Custom|FireTest
  (bind _arrow (Variables|Default|GetArrow))
  (bind _controller (Variables|Default|GetController))
  (bind _outhit (CallFunction|Linetrace (Transformation|GetWorldLocation _arrow) (Math|Vector|GetForwardVector _arrow) 5e+03 "ForOneFrame" 2.0 "(R=1.000000,G=0.000000,B=0.000000,A=1.000000)" "(R=0.000000,G=1.000000,B=0.000000,A=1.000000)"))
  (Game|Damage|ApplyDamage (.HitActor (Collision|BreakHitResult _outhit)) 1e+01 _controller (Pawn|GetControlledPawn _controller))
  (bind _returnvalue (Utilities|Time|SetTimerbyEvent (delegate Custom|FireTest) 0.1 true)))

(event Custom|Disengage
  (Utilities|Time|ClearandInvalidateTimerbyHandle (stale Custom|FireTest _returnvalue))
  (Utilities|FlowControl|Sequence
    (:then_0
      (bind _newtrack_0 (Timeline|Timeline_0 Stop)
        (:Update
          (Transformation|SetRelativeLocation (Variables|Default|GetStaticMesh) (Math|Vector|MakeVector (Math|Float|Lerp 1.4e+02 -4e+01 _newtrack_0) 0.0 0.0) false false))))
    (:then_1
      (Timeline|Timeline_0 SetNewTime))))

(event Custom|Engage
  (CallFunction|FireTest)
  (bind _newtrack_0 (Timeline|Timeline_0 PlayFromStart)
    (:Update
      (Transformation|SetRelativeLocation (Variables|Default|GetStaticMesh) (Math|Vector|MakeVector (Math|Float|Lerp 1.4e+02 -4e+01 _newtrack_0) 0.0 0.0) false false))))

(event EventHeldInteract
  (params (Invoker :type Actor%20Object%20Reference) (InvokerComponent :type Scene%20Component%20Object%20Reference) (String :type String))
  (switch string String
    (:Start
      (CallFunction|Engage))
    (:Stop
      (CallFunction|Disengage))
    (:Drop
      (CallFunction|Detachfrom))))

(event EventReachInteract
  (params (Invoker :type Actor%20Object%20Reference) (InvokerComponent :type Scene%20Component%20Object%20Reference) (Message :type String) (Player :type Player%20Controller%20Object%20Reference))
  (Development|PrintString (Utilities|String|Append "Instigator: " (Utilities|GetDisplayName Invoker) " 
Interact Event: " Message))
  (CallFunction|Attachto Invoker InvokerComponent))

(fn ConstructionScript)

(fn Attachto
  (params (ParentActor :type Actor%20Object%20Reference) (ParentComponent :type Scene%20Component%20Object%20Reference))
  (Variables|Default|SetController (Game|GetInstigatorController ParentActor))
  (CallFunction|SetPickupPhysics false)
  (Variables|Default|SetParentActor ParentActor)
  (bind _output_get (Variables|Default|SetParentComp ParentComponent))
  (Transformation|AttachComponentToComponent _output_get "None" "SnapToTarget" "SnapToTarget" "SnapToTarget" true)
  (Transformation|SetActorTransform (Transformation|GetWorldTransform _output_get)))

(fn Detachfrom
  (Development|PrintString (Utilities|GetDisplayName (Variables|Default|GetParentComp)))
  (Transformation|DetachFromActor (Variables|Default|GetParentActor) "KeepWorld" "KeepWorld" "KeepWorld")
  (CallFunction|SetPickupPhysics true))

(fn SetPickupPhysics
  (params (Physics? :type Boolean))
  (bind _base (Variables|Default|GetBase))
  (Physics|SetSimulatePhysics _base Physics?)
  (Collision|SetCollisionEnabled _base (select Physics? "QueryAndPhysics" "NoCollision")))