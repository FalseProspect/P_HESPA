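; Base pickup prop that attaches to whoever interacts with it and can be dropped, driven by interact events.
; ReachInteract disables physics and collision, then snaps the pickup to the invoker's component.
; HeldInteract routes Start and Stop to Engage and Disengage, which only print debug text, and Drop to DetachFrom.
; DetachFrom calls DetachFromActor on the stored parent actor, not the pickup, then restores physics and collision.
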(event Custom|Disengage
  (Development|PrintString "Disengage"))

(event Custom|Engage
  (Development|PrintString "Engage"))

(event EventHeldInteract
  (params (Invoker :type Actor%20Object%20Reference) (InvokerComponent :type Scene%20Component%20Object%20Reference) (String :type String))
  (switch string String
    (:Start
      (CallFunction|Engage))
    (:Stop
      (CallFunction|Disengage))
    (:Drop
      (CallFunction|Detachfrom))))

(event EventReachInteract
  (params (Invoker :type Actor%20Object%20Reference) (InvokerComponent :type Scene%20Component%20Object%20Reference) (Message :type String) (Player :type Player%20Controller%20Object%20Reference))
  (Development|PrintString (Utilities|String|Append "Instigator: " (Utilities|GetDisplayName Invoker) " 
Interact Event: " Message))
  (CallFunction|Attachto Invoker InvokerComponent))

(fn ConstructionScript)

(fn Attachto
  (params (ParentActor :type Actor%20Object%20Reference) (ParentComponent :type Scene%20Component%20Object%20Reference))
  (CallFunction|SetPickupPhysics false)
  (Variables|Default|SetParentActor ParentActor)
  (bind _output_get (Variables|Default|SetParentComp ParentComponent))
  (Transformation|AttachComponentToComponent _output_get "None" "SnapToTarget" "SnapToTarget" "SnapToTarget" true)
  (Transformation|SetActorTransform (Transformation|GetWorldTransform _output_get)))

(fn Detachfrom
  (Development|PrintString (Utilities|GetDisplayName (Variables|Default|GetParentComp)))
  (Transformation|DetachFromActor (Variables|Default|GetParentActor) "KeepWorld" "KeepWorld" "KeepWorld")
  (CallFunction|SetPickupPhysics true))

(fn SetPickupPhysics
  (params (Physics? :type Boolean))
  (bind _base (Variables|Default|GetBase))
  (Physics|SetSimulatePhysics _base Physics?)
  (Collision|SetCollisionEnabled _base (select Physics? "QueryAndPhysics" "NoCollision")))