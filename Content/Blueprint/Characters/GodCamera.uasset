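; GodCamera is a player-controlled camera pawn with axis-driven movement, mouse wheel zoom and a switch to a free camera.
; Movement input follows the actor's forward and right vectors.
; Zoom shifts a target distance seeded from the spring arm length, and a restarted timeline eases the arm toward it.
; F spawns a FreeCamera at the camera's transform if none exists, passes itself as parent pawn, and possesses it.
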(event Input|AxisEvents|InputAxisMoveForward
  (params (AxisValue :type Float%20%28single-precision%29))
  ;[1 1 1] Basic Movement
  (Pawn|Input|AddMovementInput (Transformation|GetActorForwardVector) AxisValue false))

(event Input|AxisEvents|InputAxisMoveRight
  (params (AxisValue :type Float%20%28single-precision%29))
  ;[1 1 1] Basic Movement
  (Pawn|Input|AddMovementInput (Transformation|GetActorRightVector) AxisValue false))

(event Input|MouseEvents|MouseWheelAxis
  (params (AxisValue :type Float%20%28single-precision%29))
  ;[1 1 1] Adjust Camera Zoom
  (|AdjustZoom (* AxisValue -1.0)))

(event Input|KeyboardEvents|F
  (params (Key :type Key%20Structure))
  ;[1 1 1] Toggle Free Camera
  (:Pressed
    (CallFunction|ToggleFreeCamera)))

(fn ConstructionScript
  (Variables|Default|SetZoomDist (Variables|/Script/Engine.SpringArmComponent|GetTargetArmLength (Variables|Default|GetSpringArm))))

(fn ToggleFreeCamera
  (Utilities|IsValid (Variables|Default|GetFreeCam)
    (:Is%20Valid
      _)
    (:Is%20Not%20Valid
      (bind _returnvalue (Game|SpawnActorfromClass "/Game/Blueprint/Characters/FreeCamera.FreeCamera_C" (Transformation|GetWorldTransform (Variables|Default|GetCamera)) "Undefined" 0 self 0))
      (Variables|Default|SetFreeCam _returnvalue)))
  (Pawn|Possess (Game|GetPlayerController 0) (Variables|Default|GetFreeCam)))