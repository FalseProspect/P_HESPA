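; BasicMobCharacter is a character Blueprint that handles interacting with world objects and using a held item.
; Fire/Engage, Use and Drop inputs send held or reach interaction messages with string commands.
; ReachInteraction line-traces from the camera, messages the hit actor and caches whatever is attached to Arrow1 as EquippedObject.
; HeldInteraction forwards commands to that object and detaches it on Drop; dialog-focus handling is left unfinished.
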(event Input|ActionEvents|InputActionFire/Engage
  (params (Key :type Key%20Structure))
  (bind _self self)
  (:Pressed
    (Class|BPInterInteract|HeldInteract(Message) _self _self 0 "Start"))
  (:Released
    (Class|BPInterInteract|HeldInteract(Message) _self _self 0 "Stop")))

(event Input|ActionEvents|InputActionUse
  (params (Key :type Key%20Structure))
  (bind _self self)
  (:Pressed
    (Variables|Default|SetinFocusHeld? false)
    (Class|BPInterInteract|ReachInteract(Message) _self _self 0 "Use" (Game|GetPlayerController 0))
    ;[1 1 1] If focus in not immediatly set back to true, remove dialog box
    (if (not (Variables|Default|GetinFocusHeld?))
      _)))

(event Input|ActionEvents|InputActionDrop
  (params (Key :type Key%20Structure))
  (bind _self self)
  (:Pressed
    (Class|BPInterInteract|HeldInteract(Message) _self _self 0 "Drop")))

(fn ConstructionScript)

(fn LineTraceReach
  (params (Reach :type Float%20%28single-precision%29))
  (bind _returnvalue (Game|GetPlayerCameraManager 0))
  (bind (_outhit _returnvalue_2) (CallFunction|Linetrace (Transformation|GetActorLocation _returnvalue) (Transformation|GetActorForwardVector _returnvalue) Reach (select (Variables|Debug|GetDebug) "ForDuration" "None") 1.0 "(R=1.000000,G=0.000000,B=0.000000,A=1.000000)" "(R=0.000000,G=1.000000,B=0.000000,A=1.000000)"))
  (return _outhit _returnvalue_2 (.HitActor (Collision|BreakHitResult _outhit)) (.HitComponent (Collision|BreakHitResult _outhit))))

(fn ReachInteraction
  (params (Message :type String) (Player :type Player%20Controller%20Object%20Reference))
  (bind _arrow1 (Variables|Default|GetArrow1))
  (bind _returnvalue (Components|GetChildComponent _arrow1 0))
  (Class|BPInterInteract|ReachInteract(Message) (.HitActor (CallFunction|LineTraceReach 3e+02)) self 0 Message Player)
  (Utilities|IsValid _returnvalue
    (:Is%20Valid
      (Variables|Default|SetEquippedObject (Components|GetOwner _returnvalue)))))

(fn HeldInteraction
  (params (Selection :type String))
  (Utilities|IsValid (Variables|Default|GetEquippedObject)
    (:Is%20Valid
      (Class|BPInterInteract|HeldInteract(Message) (Variables|Default|GetEquippedObject) self 0 Selection)
      (switch string Selection
        (:Drop
          (Transformation|DetachFromActor (Variables|Default|GetEquippedObject) "KeepWorld" "KeepWorld" "KeepWorld")
          (Variables|Default|SetEquippedObject 0))))))