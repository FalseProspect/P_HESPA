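; FreeCamera is a possessable free-camera Blueprint that can hand player control back to a stored parent pawn.
; Pressing F calls ToggleFreeCamera, which makes player 0's controller possess ParentPawn, or prints a warning if none is valid.
; The Fire/Engage action and right mouse button share one long line trace from the camera manager's location along its forward vector, with timed debug drawing and no use of the result.
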(event Input|ActionEvents|InputActionFire/Engage
  (params (Key :type Key%20Structure))
  (bind _returnvalue (Game|GetPlayerCameraManager 0))
  (:Pressed
    (CallFunction|Linetrace (Transformation|GetActorLocation _returnvalue) (Transformation|GetActorForwardVector _returnvalue) 1e+04 "ForDuration" 5e+01 "(R=1.000000,G=0.000000,B=0.000000,A=1.000000)" "(R=0.000000,G=1.000000,B=0.000000,A=1.000000)")))

(event Input|KeyboardEvents|F
  (params (Key :type Key%20Structure))
  (:Pressed
    (CallFunction|ToggleFreeCamera)))

(event Input|MouseEvents|RightMouseButton
  (params (Key :type Key%20Structure))
  (bind _returnvalue (Game|GetPlayerCameraManager 0))
  (:Pressed
    (CallFunction|Linetrace (Transformation|GetActorLocation _returnvalue) (Transformation|GetActorForwardVector _returnvalue) 1e+04 "ForDuration" 5e+01 "(R=1.000000,G=0.000000,B=0.000000,A=1.000000)" "(R=0.000000,G=1.000000,B=0.000000,A=1.000000)")))

(fn ConstructionScript)

(fn ToggleFreeCamera
  (bind _parentpawn (Variables|Default|GetParentPawn))
  (Utilities|IsValid _parentpawn
    (:Is%20Valid
      (Pawn|Possess (Game|GetPlayerController 0) _parentpawn))
    (:Is%20Not%20Valid
      (Development|PrintString "No parent pawn set" true true "(R=1.000000,G=1.000000,B=0.000000,A=1.000000)"))))